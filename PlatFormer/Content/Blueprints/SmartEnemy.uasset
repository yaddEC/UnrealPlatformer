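; Enemy character that damages whatever it hits and can be defeated by hits to its head from Player-tagged components.
; Each head hit removes one Health, with a DoOnce and short delayed reset debouncing repeated collisions.
; At one Health it sets the LowLife blackboard key for its AI and changes walk speed.
; At zero it spawns a OneUp at its transform and destroys itself.
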(event OnComponentHit(HeadCollision)
  (params (HitComponent :type Primitive%20Component%20Object%20Reference) (OtherActor :type Actor%20Object%20Reference) (OtherComp :type Primitive%20Component%20Object%20Reference) (NormalImpulse :type Vector :default "0, 0, 0") (Hit :type Hit%20Result%20Structure%20%28by%20ref%29))
  ;[1 1 1] Damage and Despawn
  (if (Components|ComponentHasTag OtherComp "Player")
    (Utilities|FlowControl|DoOnce false :!label _label
      (:Completed
        (Variables|Default|SetHealth (- (Variables|Default|GetHealth) 1))
        (if (== (Variables|Default|GetHealth) 1)
          (AI|Components|Blackboard|SetValueasBool (AI|GetBlackboard self) (Utilities|Name|MakeLiteralName "LowLife") true)
          (Variables|/Script/Engine.CharacterMovementComponent|SetMaxWalkSpeed (Variables|Character|GetCharacterMovement) 3e+02)
          (Utilities|FlowControl|Delay 0.2 :!label _label_2)
          (goto _label Reset)
          (elif (<= (Variables|Default|GetHealth) 0)
            (Game|SpawnActorfromClass "/Game/Blueprints/OneUp.OneUp_C" (Transformation|GetActorTransform self) "Undefined" 0 0)
            (Actor|DestroyActor)
            (else
              (goto _label_2))))))))

(event EventBeginPlay
  ;[1 1 1] Inflict Damage
)

(event Collision|EventHit
  (params (MyComp :type Primitive%20Component%20Object%20Reference) (Other :type Actor%20Object%20Reference) (OtherComp :type Primitive%20Component%20Object%20Reference) (bSelfMoved :type Boolean) (HitLocation :type Vector :default "0, 0, 0") (HitNormal :type Vector :default "0, 0, 0") (NormalImpulse :type Vector :default "0, 0, 0") (Hit :type Hit%20Result%20Structure%20%28by%20ref%29))
  ;[1 1 1] Inflict Damage
  (Game|Damage|ApplyDamage Other 2e+01 0 0))

(fn ConstructionScript)