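; Moving platform actor that slides its cube mesh back and forth from BeginPlay using the Move timeline.
; Each update sets the cube's relative location to a lerp from the Slide track toward its current location, with a tiny delta-time alpha, so it closely follows the track.
; A three-second Delay on the Update path then toggles Loop to alternate between reversing and playing the timeline.
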(event EventBeginPlay
  (bind _slide (Timeline|Move Play)
    (:Update
      (Transformation|SetRelativeLocation (Variables|Default|Get1M_Cube) (Math|Vector|Lerp(Vector) _slide (Variables|/Script/Engine.SceneComponent|GetRelativeLocation (Variables|Default|Get1M_Cube)) (* (Utilities|Time|GetWorldDeltaSeconds) 0.0001)) false false)
      (Utilities|FlowControl|Delay 3.0)
      (if (Variables|Default|GetLoop)
        (Variables|Default|SetLoop false)
        (Timeline|Move Reverse)
        (else
          (Variables|Default|SetLoop true)
          (Timeline|Move Play))))))

(event Collision|EventActorBeginOverlap
  (params (OtherActor :type Actor%20Object%20Reference)))

(event EventTick
  (params (DeltaSeconds :type Float%20%28single-precision%29)))

(fn ConstructionScript)