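; Behavior tree task that heals a SmartEnemy pawn after a counted delay.
; Each execution increments the HealingPercent blackboard counter and finishes as failed until the counter reaches its threshold.
; At the threshold it sets the enemy's walk speed, adds one Health, clears IsLow, resets the counter and finishes successfully.
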(event EventReceiveExecuteAI
  (params (OwnerController :type AI%20Controller%20Object%20Reference) (ControlledPawn :type Pawn%20Object%20Reference))
  (bind _healingpercent (Variables|Default|GetHealingPercent))
  (bind _returnvalue (Class|BTFunctionLibrary|GetBlackboardValueasInt _healingpercent))
  (if (>= _returnvalue 300)
    (bind _assmart_enemy (Utilities|Casting|CastToSmartEnemy ControlledPawn))
    (Variables|/Script/Engine.CharacterMovementComponent|SetMaxWalkSpeed (Variables|/Script/Engine.Character|GetCharacterMovement _assmart_enemy) 6e+02)
    (Variables|/Game/Blueprints/SmartEnemy.SmartEnemy_C|SetHealth _assmart_enemy (+ (Variables|/Game/Blueprints/SmartEnemy.SmartEnemy_C|GetHealth _assmart_enemy) 1))
    (Class|BTFunctionLibrary|SetBlackboardValueasBool (Variables|Default|GetIsLow) false)
    (Class|BTFunctionLibrary|SetBlackboardValueasInt (Variables|Default|GetHealingPercent))
    (AI|BehaviorTree|FinishExecute true)
    (else
      (Class|BTFunctionLibrary|SetBlackboardValueasInt _healingpercent (+ _returnvalue 1))
      (AI|BehaviorTree|FinishExecute false))))