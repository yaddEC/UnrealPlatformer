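; Player character Blueprint with axis-driven movement and look, jumping, damage handling and a toggle between first and third person cameras.
; Damage lowers Health behind a half-second re-entry lock and updates the progress bar on the HUD created at BeginPlay.
; Wall jumping is unfinished: Tick traces while falling but always clears WallSlide, slide logic is disconnected, and JumpCounter's limit check is unused.
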(event EventOnLanded
  (params (Hit :type Hit%20Result%20Structure%20%28by%20ref%29))
  ;[1 1 1] Player Jump
  (Variables|Default|SetJumpCounter 0))

(event EventTick
  (params (DeltaSeconds :type Float%20%28single-precision%29))
  (bind _returnvalue (Transformation|GetActorLocation))
  ;[1 1 1] Wall Jump
  (if (AI|Components|NavMovement|IsFalling (Variables|Character|GetCharacterMovement))
    (bind (_outhit _returnvalue_2) (Collision|LineTraceByChannel _returnvalue (* _returnvalue (* (Transformation|GetActorForwardVector) 7e+01)) "TraceTypeQuery1" false 0 "None"))
    (if _returnvalue_2
      (Variables|Default|SetwallSlide false)
      (else
        (Variables|Default|SetwallSlide false :!label _label)))
    (else
      (goto _label))))

(event Game|Damage|EventAnyDamage
  (params (Damage :type Float%20%28single-precision%29) (DamageType :type Damage%20Type%20Object%20Reference) (InstigatedBy :type Controller%20Object%20Reference) (DamageCauser :type Actor%20Object%20Reference))
  ;[1 1 1] Get Damaged
  (Utilities|FlowControl|DoOnce false :!label _label
    (:Completed
      (bind _output_get (Variables|Default|SetHealth (- (Variables|Default|GetHealth) (Math|Float|Truncate Damage))))
      (Development|PrintString (Utilities|String|ToString(Integer) _output_get))
      (Progress|SetPercent (Variables|/Game/UI/GameHUD.GameHUD_C|GetProgressBar_1 (Variables|Default|GetPlayerHUD)) (/ (Math|Conversions|ToFloat(Integer) (Variables|Default|GetHealth)) 1e+02))
      (Utilities|FlowControl|Delay 0.5)
      (goto _label Reset))))

(event EventBeginPlay
  ;[1 1 1] GameHUD
  (bind _returnvalue (UserInterface|CreateWidget "/Game/UI/GameHUD.GameHUD_C" (Game|GetPlayerController 0)))
  (bind _output_get (Variables|Default|SetPlayerHUD _returnvalue))
  (UserInterface|Viewport|AddtoViewport _output_get 0))

(event Input|ActionEvents|InputActionJump
  (params (Key :type Key%20Structure :default "None"))
  ;[1 1 1] Player Jump
  (:Pressed
    (if (Variables|Default|GetwallSlide)
      (Character|LaunchCharacter (* (* (Transformation|GetActorForwardVector) -5e+02) "0, 0,1000.000000") false false)
      (else
        (Variables|Default|SetJumpCounter (+ (Variables|Default|GetJumpCounter) 1))
        (Character|Jump))))
  (:Released
    (Character|StopJumping)))

(event Input|AxisEvents|InputAxisForward/Backward
  (params (AxisValue :type Float%20%28single-precision%29))
  ;[1 1 1] Basic Player Movement
  (Pawn|Input|AddMovementInput (Math|Vector|GetForwardVector (Math|Rotator|MakeRotator 0.0 0.0 (.Yaw (Math|Rotator|BreakRotator (Pawn|GetControlRotation :!class /Script/Engine.Pawn))))) AxisValue false))

(event Input|AxisEvents|InputAxisRight/Left
  (params (AxisValue :type Float%20%28single-precision%29))
  ;[1 1 1] Basic Player Movement
  (Pawn|Input|AddMovementInput (Math|Vector|GetRightVector (Math|Rotator|MakeRotator 0.0 0.0 (.Yaw (Math|Rotator|BreakRotator (Pawn|GetControlRotation :!class /Script/Engine.Pawn))))) AxisValue false))

(event Input|AxisEvents|InputAxisTurnUpDownCam
  (params (AxisValue :type Float%20%28single-precision%29))
  ;[1 1 1] Basic Camera
  (Pawn|Input|AddControllerPitchInput AxisValue))

(event Input|AxisEvents|InputAxisTurnLeftRightCam
  (params (AxisValue :type Float%20%28single-precision%29))
  ;[1 1 1] Basic Camera
  (Pawn|Input|AddControllerYawInput AxisValue))

(event Input|KeyboardEvents|K
  (params (Key :type Key%20Structure :default "None"))
  ;[1 1 1] Setup First or Third camera
  (:Pressed
    (Utilities|FlowControl|FlipFlop
      (:A
        (Components|Activation|SetActive (Variables|Default|GetFirstPersonCamera) false false)
        (Components|Activation|SetActive (Variables|Default|GetThirdCamera) true false))
      (:B
        (Components|Activation|SetActive (Variables|Default|GetThirdCamera) false false)
        (Components|Activation|SetActive (Variables|Default|GetFirstPersonCamera) true false)))))

(fn ConstructionScript)