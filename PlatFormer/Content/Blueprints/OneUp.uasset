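; OneUp is a health pickup actor that restores a fixed amount of player health.
; When a component tagged Player begins overlapping its Sphere, it casts the other actor to Player and adds to Health without clamping.
; It then writes the new health fraction directly to the player HUD's progress bar and destroys itself.
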(event OnComponentBeginOverlap(Sphere)
  (params (OverlappedComponent :type Primitive%20Component%20Object%20Reference) (OtherActor :type Actor%20Object%20Reference) (OtherComp :type Primitive%20Component%20Object%20Reference) (OtherBodyIndex :type Integer) (bFromSweep :type Boolean) (SweepResult :type Hit%20Result%20Structure%20%28by%20ref%29))
  (if (Components|ComponentHasTag OtherComp "Player")
    (bind _asplayer (Utilities|Casting|CastToPlayer OtherActor))
    (Variables|/Game/Blueprints/Player.Player_C|SetHealth _asplayer (+ (Variables|/Game/Blueprints/Player.Player_C|GetHealth _asplayer) 20))
    (Progress|SetPercent (Variables|/Game/UI/GameHUD.GameHUD_C|GetProgressBar_1 (Variables|/Game/Blueprints/Player.Player_C|GetPlayerHUD _asplayer)) (/ (Math|Conversions|ToFloat(Integer) (Variables|/Game/Blueprints/Player.Player_C|GetHealth _asplayer)) 1e+02))
    (Actor|DestroyActor)))

(fn ConstructionScript)