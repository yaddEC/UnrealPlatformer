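; Behavior tree task that picks a flee destination for an AI pawn, directly away from the player.
; It reads PlayerLocation from the Blackboard and projects a point a fixed distance opposite the look-at direction, keeping the pawn's current height.
; The result is written to TargetLocation and the task finishes successfully at once, without moving the pawn itself.
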(event EventReceiveExecuteAI
  (params (OwnerController :type AI%20Controller%20Object%20Reference) (ControlledPawn :type Pawn%20Object%20Reference))
  (bind _returnvalue (Transformation|GetActorLocation ControlledPawn))
  (bind _playerlocation (Variables|Default|GetPlayerLocation))
  (bind _returnvalue_2 (Class|BTFunctionLibrary|GetBlackboardValueasVector _playerlocation))
  (bind _returnvalue_3 (Math|Rotator|FindLookatRotation _returnvalue _returnvalue_2))
  (bind _returnvalue_4 (Math|Vector|GetForwardVector _returnvalue_3))
  (bind _returnvalue_5 (* _returnvalue_4 -5e+02))
  (bind _returnvalue_6 (+ _returnvalue _returnvalue_5))
  (bind (_x _y) (Math|Vector|BreakVector _returnvalue_6))
  (AI|BehaviorTree|SetBlackboardValueasVector (Variables|Default|GetTargetLocation) (Math|Vector|MakeVector _x _y (.Z (Math|Vector|BreakVector _returnvalue))))
  (AI|BehaviorTree|FinishExecute true))